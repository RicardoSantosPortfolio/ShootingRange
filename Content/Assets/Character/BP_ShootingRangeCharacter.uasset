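; Player character for a shooting range, with movement, controller-driven look and a gun.
; BeginPlay spawns a BP_Gun2 and snaps it to GunLocation; each Shoot press fires it along a long line from the camera's forward vector.
; CanShoot limits firing to one shot per press, and each shot notifies VariablesSublevel to count it.
; Look axis names are crossed: LookUp drives yaw and LookRight drives pitch.
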(event `self.ReceiveBeginPlay`
  (bind _returnvalue (`|SpawnActorFromClass` "/Game/Assets/Gun2/BP_Gun2.BP_Gun2_C" (`KismetMathLibrary.MakeTransform` (0.0 0.0 0.0)) "Undefined" "OverrideRootScale" null null))
  (bind _output_get (set `self.EquippedGun` _returnvalue))
  (`self.K2_AttachToComponent` _output_get (`self.GunLocation`) "None" "SnapToTarget" "SnapToTarget" "KeepRelative" true))

(event `InputAction|Shoot`
  (params (Key :type "Key Structure"))
  (bind _camera (`self.Camera`))
  (bind _returnvalue (`SceneComponent.K2_GetComponentLocation` _camera))
  (:`Pressed`
    (if (`self.CanShoot`)
      (message `/Game/IGlobalVariables.AddToShotsFired` (`GameplayStatics.GetStreamingLevel` "VariablesSublevel"))
      (`/Game/Assets/BP_GenericGun.Shoot` (`self.EquippedGun`) _returnvalue (+ _returnvalue (* (`SceneComponent.GetForwardVector` _camera) 5000000.0)))
      (set `self.CanShoot` false)))
  (:`Released`
    (set `self.CanShoot` true)))

(event `InputAxis|MoveForward`
  (params (AxisValue :type "Float (single-precision)"))
  (`self.AddMovementInput` (`self.GetActorForwardVector`) AxisValue))

(event `InputAxis|MoveRight`
  (params (AxisValue :type "Float (single-precision)"))
  (`self.AddMovementInput` (`self.GetActorRightVector`) AxisValue))

(event `InputAxis|LookUp`
  (params (AxisValue :type "Float (single-precision)"))
  (`self.AddControllerYawInput` AxisValue))

(event `InputAxis|LookRight`
  (params (AxisValue :type "Float (single-precision)"))
  (`self.AddControllerPitchInput` AxisValue))

(fn `UserConstructionScript`)