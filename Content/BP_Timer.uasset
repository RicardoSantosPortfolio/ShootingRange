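; BP_Timer is an in-world game countdown actor that shows the remaining time on TimerText.
; ResetTimer restores the total time and enables counting, while Tick uses a latent Delay to decrement it once per second and refreshes text through SecondsToText.
; At zero, it disables itself and every TargetSpawner, then restores the visibility and collision of the BotaoIniciar start button.
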(event `self.ReceiveBeginPlay`
  (`TextRenderComponent.K2_SetText` (`self.TimerText`) (`self.SecondsToText` (`self.GameTimeInSeconds`))))

(event `self.ReceiveTick`
  (params (DeltaSeconds :type "Float (single-precision)"))
  (bind _gametimeinseconds (`self.GameTimeInSeconds`))
  (bind _botao (`/Game/BotaoIniciar.Botao` (`self.BotaoIniciar`)))
  (`TextRenderComponent.K2_SetText` (`self.TimerText`) (`self.SecondsToText` (`self.GameTimeInSeconds`)))
  (`|ExecutionSequence`
    (:`then_0`
      (if (== 0.0 (`self.GameTimeInSeconds`))
        (set `self.Enabled` false)
        (`SceneComponent.SetVisibility` _botao true true)
        (`PrimitiveComponent.SetCollisionEnabled` _botao "QueryAndPhysics")
        (bind _outactors (`GameplayStatics.GetAllActorsOfClass` "/Game/Assets/TargetCreator/TargetSpawner.TargetSpawner_C"))
        (for _array_element _outactors
          (set `/Game/Assets/TargetCreator/TargetSpawner.Enabled` false _array_element))))
    (:`then_1`
      (if (`self.Enabled`)
        (`TextRenderComponent.K2_SetText` (`self.TimerText`) (`self.SecondsToText` _gametimeinseconds))
        (`KismetSystemLibrary.Delay` 1.0)
        (`/Engine/EditorBlueprintResources/StandardMacros.DecrementFloat` _gametimeinseconds)))))

(fn `ResetTimer`
  (set `self.GameTimeInSeconds` (`self.TotalGameTime`))
  (set `self.Enabled` true))

(fn `UserConstructionScript`)